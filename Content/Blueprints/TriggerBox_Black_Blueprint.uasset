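; Clickable trigger box that selects the black side for the local player and opens the black chess selection screen.
; On click, it checks the ChessBoardManager status and player state, sets the player, and suspends the status during the transition.
; It clears widgets, blends the camera to the black selection view, then after a delay shows SelectChess_Black with manager, camera and BGM references and restores the status.
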(event `self.ReceiveActorOnClicked`
  (params (ButtonPressed :type "Key Structure"))
  (bind _returnvalue (`self.GetCurrentStatus` (`.ChessBoardManager` (`self.ChessBoardManager`))))
  ;[1 1 1] 判断是否满足条件
  (if (== _returnvalue 1)
    (bind _returnvalue_2 (`self.GetSelfPlayer` (`.ChessBoardManager` (`self.ChessBoardManager`))))
    (if (== _returnvalue_2 2)
      (`self.SetCurrentStatus` (`.ChessBoardManager` (`self.ChessBoardManager`)) -1)
      (`self.SetSelfPlayer` (`.ChessBoardManager` (`self.ChessBoardManager`)) true)
      ;[1 1 1] 变换UI
      (`WidgetLayoutLibrary.RemoveAllWidgets`)
      (`PlayerController.SetViewTargetWithBlend` (`GameplayStatics.GetPlayerController` 0) (`self.SelectChess_Black`) 1.0 "VTBlend_Cubic" 0.0 false)
      (`KismetSystemLibrary.Delay` 1.0)
      (bind _returnvalue_3 (`|CreateWidget` "/Game/UI/SinglePlay/SelectChess_Black.SelectChess_Black_C" (`GameplayStatics.GetPlayerController` 0)))
      (bind _this (`/Game/UI/SinglePlay/SelectChess_Black.InitUI` _returnvalue_3 (`.ChessBoardManager` (`self.ChessBoardManager`)) (`self.PlayCamera_Black`) (`self.BGM`)))
      (`UserWidget.AddToViewport` _this 0)
      (`self.SetCurrentStatus` (`.ChessBoardManager` (`self.ChessBoardManager`)) 1))))

(fn `UserConstructionScript`)