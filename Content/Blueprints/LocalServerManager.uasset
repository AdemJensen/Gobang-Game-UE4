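; LocalServerManager is an actor that runs a TCP socket server for a single client at a configured IP and port.
; Connection events route by server or client type, binding message reception once the server starts and closing any client that connects while a session is held.
; It stores the client's SessionID for SendData and Kick, and relays connects, disconnects and incoming messages through its own dispatchers.
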(event `self.Configure`
  (params (Ip :type String) (Port :type Integer))
  (set `self.Ip` Ip)
  (set `self.Port` Port))

(event `self.StartUp`
  (`SocketServerBPLibrary.startTCPServer` (`SocketServerBPLibrary.getSocketServerTarget`) (`self.Ip`) (`self.Port`) "E_SAB")
  (add `SocketServerBPLibrary.onsocketServerConnectionEventDelegate` (`SocketServerBPLibrary.getSocketServerTarget`) (delegate `OnNewConnectionEvent`))
  (`KismetSystemLibrary.PrintString` "Socket server is online."))

(event `OnNewConnectionEvent`
  (params (type :type "EServerSocketConnectionEventType Enum" :default "E_Server") (success :type Boolean) (message :type String) (sessionID :type String))
  (switch `EServerSocketConnectionEventType` type
    (:`E_Server`
      (`self.Server Connection Event` success message))
    (:`E_Client`
      (`self.Client Connection Event` success sessionID message))))

(event `self.ShutDown`
  (`SocketServerBPLibrary.stopTCPServer` (`SocketServerBPLibrary.getSocketServerTarget`)))

(event `Server Connection Event`
  (params (bSuccess :type Boolean) (Message :type String))
  ;[1 1 1] Message Listener is created if TCP Server is Started successfully.
  (`KismetSystemLibrary.PrintString` (`KismetStringLibrary.Concat_StrStr` (`KismetStringLibrary.Conv_BoolToString` bSuccess) " | " Message))
  (if bSuccess
    ;;[1 1 1] Message from client
    (add `SocketServerBPLibrary.onserverReceiveTCPMessageEventDelegate` (`SocketServerBPLibrary.getSocketServerTarget`) (delegate `OnReceiveMessage`))))

(event `OnReceiveMessage`
  (params (sessionID :type String) (message :type String) (byteArray :type "Array of Byte (by ref)"))
  ;[1 1 1] Message Listener is created if TCP Server is Started successfully.
  ;;[1 1 1] Message from client
  (`KismetSystemLibrary.PrintString` (`KismetStringLibrary.Concat_StrStr` sessionID " | " message))
  (`self.OnIncommingMessage` message))

(event `Client Connection Event`
  (params (bSuccess :type Boolean) (`Session Id` :type String) (Message :type String))
  ;[1 1 1] New Client connected / Disconnected (Rusulted on 'Success'), Each Client has a SessionID that should be saved to send messages to this Client back.
  (`KismetSystemLibrary.PrintString` (`KismetStringLibrary.Concat_StrStr` (`KismetStringLibrary.Conv_BoolToString` bSuccess) " | " `Session Id` " | " Message))
  (if bSuccess
    ;;[1 1 1] If already connected, close immediately.
    (bind _connected (`self.IsConnected`))
    (if _connected
      (`SocketServerBPLibrary.closeTCPClientConnection` (`SocketServerBPLibrary.getSocketServerTarget`) `Session Id`)
      (else
        (set `self.Session` `Session Id`)
        (`self.OnClientConnected`)))
    (else
      (set `self.Session` "")
      (`self.OnClientDisconnected`))))

(fn `IsConnected`
  (returns (Connected :type Boolean))
  (return (> (`KismetStringLibrary.Len` (`self.Session`)) 0)))

(fn `Kick`
  (if (> (`KismetStringLibrary.Len` (`self.Session`)) 0)
    (`SocketServerBPLibrary.closeTCPClientConnection` (`SocketServerBPLibrary.getSocketServerTarget`) (`self.Session`))
    (set `self.Session` "")))

(fn `Send Data`
  (params (Content :type String))
  (returns (Success :type Boolean))
  (bind _connected (`self.IsConnected`))
  (if _connected
    (`SocketServerBPLibrary.socketServerSendTCPMessage` (`SocketServerBPLibrary.getSocketServerTarget`) (`|MakeArray` (`self.Session`)) "" (`TcpSocketConnection.Conv_StringToBytes` Content) true false)
    (return true)
    (else
      (return false))))

(fn `UserConstructionScript`)