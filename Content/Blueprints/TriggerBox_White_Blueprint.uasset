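; Clickable trigger box that switches the local player from one side to white in the chess board's selection screen.
; A click acts only in status 1 with the self-player flag set, and is blocked when ban mode is on at higher AI difficulty.
; It clears the flag, blends the camera to the white selection view and swaps in the SelectChess_White widget, suspending the manager's status until the transition finishes.
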(event `self.ReceiveActorOnClicked`
  (params (ButtonPressed :type "Key Structure"))
  (bind _chessboardmanager (`self.ChessBoardManager`))
  (bind _returnvalue (`ChessBoardManager.GetCurrentStatus` (`self.ChessBoardManager`)))
  ;[1 1 1] 判断是否满足条件
  (if (== _returnvalue 1)
    (bind _returnvalue_2 (`ChessBoardManager.GetSelfPlayer` (`self.ChessBoardManager`)))
    (if (== _returnvalue_2 1)
      (bind _returnvalue_3 (`ChessBoardManager.GetAiDifficulty` _chessboardmanager))
      (bind _returnvalue_4 (`ChessBoardManager.GetBanMode` _chessboardmanager))
      (if (not (and _returnvalue_4 (> _returnvalue_3 2)))
        (`ChessBoardManager.SetCurrentStatus` (`self.ChessBoardManager`) -1)
        (`ChessBoardManager.SetSelfPlayer` (`self.ChessBoardManager`) false)
        ;[1 1 1] 变换UI
        (`WidgetLayoutLibrary.RemoveAllWidgets`)
        (`PlayerController.SetViewTargetWithBlend` (`GameplayStatics.GetPlayerController` 0) (`self.SelectChess_White`) 1.0 "VTBlend_Cubic" 0.0 false)
        (`KismetSystemLibrary.Delay` 1.0)
        (bind _returnvalue_5 (`|CreateWidget` "/Game/UI/SelectChess_White.SelectChess_White_C" (`GameplayStatics.GetPlayerController` 0)))
        (bind _this (`/Game/UI/SelectChess_White.initUI` _returnvalue_5 (`self.ChessBoardManager`) (`self.PlayCamera_White`) (`self.BGM`)))
        (`UserWidget.AddToViewport` _this 0)
        (`ChessBoardManager.SetCurrentStatus` (`self.ChessBoardManager`) 1)))))

(fn `UserConstructionScript`)