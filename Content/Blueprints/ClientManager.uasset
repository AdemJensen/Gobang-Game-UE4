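; ClientManager is a Blueprint actor that wraps a TCP connection component as a client for exchanging string messages with a server.
; Configure stores the IP and port, StartUp connects unless a connection ID is already held, and ShutDown disconnects it.
; Connection, disconnection and incoming-message callbacks print debug text and re-broadcast through dispatchers, with received bytes decoded to strings.
; SendData converts content to bytes, sends it when connected and returns the result.
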(event `self.ReceiveBeginPlay`)

(event `self.Configure`
  (params (Ip :type String) (Port :type Integer))
  (set `self.Ip` Ip)
  (set `self.Port` Port))

(event `self.StartUp`
  (bind _connected (`self.IsConnected`))
  (if (not _connected)
    (bind _connectionid (`TcpSocketConnection.Connect` (`self.TCP Connection`) (`self.Ip`) (`self.Port`) (delegate `Disconnected`) (delegate `Connected`) (delegate `Message Received`)))
    (set `self.ConnectionId` _connectionid)))

(event `Disconnected`
  (params (ConnectionId :type Integer))
  (`KismetSystemLibrary.PrintString` "Disonnected!")
  (`self.OnDisconnected`))

(event `Connected`
  (params (ConnectionId :type Integer))
  (`KismetSystemLibrary.PrintString` "Connected!")
  (`self.OnConnected`))

(event `Message Received`
  (params (ConnectionId :type Integer) (Message :type "Array of Byte (by ref)"))
  (bind _returnvalue (`TcpSocketConnection.Message_ReadString` Message (`KismetArrayLibrary.Array_Length` Message)))
  (`KismetSystemLibrary.PrintString` _returnvalue)
  (`self.OnIncommingMessage` _returnvalue))

(event `self.ShutDown`
  (bind _connected (`self.IsConnected`))
  (if _connected
    (`TcpSocketConnection.Disconnect` (`self.TCP Connection`) (`self.ConnectionId`))))

(fn `IsConnected`
  (returns (Connected :type Boolean))
  (return (>= (`self.ConnectionId`) 0)))

(fn `Send Data`
  (params (Content :type String))
  (returns (Success :type Boolean))
  (bind _connected (`self.IsConnected`))
  (if _connected
    (bind _returnvalue (`TcpSocketConnection.SendData` (`self.TCP Connection`) (`self.ConnectionId`) (`TcpSocketConnection.Conv_StringToBytes` Content)))
    (`KismetSystemLibrary.PrintText` (`|FormatText` "[Client {Num}] Sent result: {result}" (`self.ConnectionId`) (`KismetTextLibrary.Conv_BoolToText` _returnvalue)))
    (return _returnvalue)
    (else
      (return false))))

(fn `UserConstructionScript`)